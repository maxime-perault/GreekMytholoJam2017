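; Stairs Blueprint that, when activable, drops its stairs below their placed position at BeginPlay and stores that lowered spot.
; ActivateStairs plays a Wwise sound and a timeline that offsets the stairs from the stored position; DesactivateStairs reverses it.
; While reversing, the location is computed as track value minus stored position, unlike the forward sum.
; The construction script, rather than BeginPlay, posts fire audio at four fire bowl locations.
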(event Custom|ActivateStairs
  (bind _stairs_pos (Variables|Default|Getstairs_pos))
  (Class|AkGameplayStatics|PostEvent "/Game/Wwise/Play_sound_blossoming_tree_2.Play_sound_blossoming_tree_2" self false)
  (bind _newtrack_1 (Timeline|Timeline_1 Play)
    (:Update
      (if (Class|TimelineComponent|IsReversing (Variables|Default|GetTimeline_1))
        (Transformation|SetWorldLocation (Variables|Default|GetStairs) (- _newtrack_1 _stairs_pos) false false)
        (else
          (Transformation|SetWorldLocation (Variables|Default|GetStairs) (+ _stairs_pos _newtrack_1) false false))))))

(event Custom|DesactivateStairs
  (bind _stairs_pos (Variables|Default|Getstairs_pos))
  (bind _newtrack_1 (Timeline|Timeline_1 Reverse)
    (:Update
      (if (Class|TimelineComponent|IsReversing (Variables|Default|GetTimeline_1))
        (Transformation|SetWorldLocation (Variables|Default|GetStairs) (- _newtrack_1 _stairs_pos) false false)
        (else
          (Transformation|SetWorldLocation (Variables|Default|GetStairs) (+ _stairs_pos _newtrack_1) false false))))))

(event EventBeginPlay
  (if (Variables|Default|GetisActivable)
    (Transformation|SetWorldLocation (Variables|Default|GetStairs) (+ (Transformation|GetWorldLocation (Variables|Default|GetStairs)) (/ "0, 0,-850.000000" 1.0)) false false)
    (Variables|Default|Setstairs_pos (Transformation|GetWorldLocation (Variables|Default|GetStairs)))))

(fn ConstructionScript
  (for _array_element (Utilities|Array|MakeArray (Variables|Default|GetFireBowlLeftTop) (Variables|Default|GetFireBowlRightTop) (Variables|Default|GetFireBowlLeftBottom) (Variables|Default|GetFireBowlRightBottom))
    (Class|AkGameplayStatics|PostEventatLocation "/Game/Wwise/Play_Fire.Play_Fire" (Transformation|GetWorldLocation _array_element) "0, 0, 0")))