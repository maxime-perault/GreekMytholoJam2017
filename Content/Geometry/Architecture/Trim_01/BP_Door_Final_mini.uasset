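; Interactable door that plays a Wwise opening sound and moves vertically when interacted with using one specific Partition enum value.
; BeginPlay scales the timeline's play rate by the inverse of OpenTime.
; Each timeline update adds a world Z offset of one minus a delta-time step based on OpenHeight and OpenTime, rather than interpolating a curve.
; It always allows interaction, exposes its Scene component as the target, and has no closing logic.
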(event EventBeginPlay
  (Components|Timeline|SetPlayRate (Variables|Default|GetTimeline_Open) (/ 1.0 (Variables|Default|GetOpenTime))))

(event Collision|EventActorBeginOverlap
  (params (OtherActor :type Actor%20Object%20Reference)))

(event EventTick
  (params (DeltaSeconds :type Float%20%28single-precision%29)))

(event EventInteract
  (params (Partition :type PartitionIDs%20Enum :default "NewEnumerator0"))
  (if (Utilities|Enum|Equal(Enum) Partition "NewEnumerator6")
    (Class|AkGameplayStatics|PostEvent "/Game/Wwise/Play_sound_obstacle_door_opens.Play_sound_obstacle_door_opens" self false)
    (Timeline|Timeline_Open Play
      (:Update
        (Transformation|AddActorWorldOffset self (Math|Vector|MakeVector 0.0 0.0 (- 1.0 (* (/ (Variables|Default|GetOpenHeight) (Variables|Default|GetOpenTime)) (Utilities|Time|GetWorldDeltaSeconds)))))))))

(fn ConstructionScript)

(fn CanInteract
  (return true))

(fn GetTarget
  (return (Variables|Default|GetScene)))