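; Three-pressure-plate puzzle prop that activates a referenced Fog object when all three plates are held at once.
; Each box overlap sets that plate's flag and plays its timeline; ending the overlap clears it and reverses.
; Timeline updates move the mesh by adding or subtracting the track value from its current location.
; Every forward update checks all three flags, so Fog.ActivatePlate can fire repeatedly.
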(event OnComponentBeginOverlap(Box03)
  (params (OverlappedComponent :type Primitive%20Component%20Object%20Reference) (OtherActor :type Actor%20Object%20Reference) (OtherComp :type Primitive%20Component%20Object%20Reference) (OtherBodyIndex :type Integer) (bFromSweep :type Boolean) (SweepResult :type Hit%20Result%20Structure%20%28by%20ref%29))
  (bind _sm_plate03 (Variables|Default|GetSM_Plate03))
  (bind _returnvalue (Transformation|GetWorldLocation _sm_plate03))
  (Variables|Default|SetIsPlate03 true)
  (bind _newtrack_1 (Timeline|Timeline_2 Play)
    (:Update
      (if (Class|TimelineComponent|IsReversing (Variables|Default|GetTimeline_2))
        (Transformation|SetWorldLocation (Variables|Default|GetSM_Plate03) (- _returnvalue _newtrack_1) false false)
        (else
          (Transformation|SetWorldLocation (Variables|Default|GetSM_Plate03) (+ _returnvalue _newtrack_1) false false)
          (if (Math|Boolean|ANDBoolean (Variables|Default|GetIsPlate01) (Variables|Default|GetIsPlate02) (Variables|Default|GetIsPlate03))
            (Default|ActivatePlate (Variables|Default|GetFog))))))))

(event OnComponentEndOverlap(Box03)
  (params (OverlappedComponent :type Primitive%20Component%20Object%20Reference) (OtherActor :type Actor%20Object%20Reference) (OtherComp :type Primitive%20Component%20Object%20Reference) (OtherBodyIndex :type Integer))
  (bind _sm_plate03 (Variables|Default|GetSM_Plate03))
  (bind _returnvalue (Transformation|GetWorldLocation _sm_plate03))
  (Variables|Default|SetIsPlate03 false)
  (bind _newtrack_1 (Timeline|Timeline_2 Reverse)
    (:Update
      (if (Class|TimelineComponent|IsReversing (Variables|Default|GetTimeline_2))
        (Transformation|SetWorldLocation (Variables|Default|GetSM_Plate03) (- _returnvalue _newtrack_1) false false)
        (else
          (Transformation|SetWorldLocation (Variables|Default|GetSM_Plate03) (+ _returnvalue _newtrack_1) false false)
          (if (Math|Boolean|ANDBoolean (Variables|Default|GetIsPlate01) (Variables|Default|GetIsPlate02) (Variables|Default|GetIsPlate03))
            (Default|ActivatePlate (Variables|Default|GetFog))))))))

(event OnComponentBeginOverlap(Box02)
  (params (OverlappedComponent :type Primitive%20Component%20Object%20Reference) (OtherActor :type Actor%20Object%20Reference) (OtherComp :type Primitive%20Component%20Object%20Reference) (OtherBodyIndex :type Integer) (bFromSweep :type Boolean) (SweepResult :type Hit%20Result%20Structure%20%28by%20ref%29))
  (bind _sm_plate02 (Variables|Default|GetSM_Plate02))
  (bind _returnvalue (Transformation|GetWorldLocation _sm_plate02))
  (Variables|Default|SetIsPlate02 true)
  (bind _newtrack_1 (Timeline|Timeline_0 Play)
    (:Update
      (if (Class|TimelineComponent|IsReversing (Variables|Default|GetTimeline_0))
        (Transformation|SetWorldLocation (Variables|Default|GetSM_Plate02) (- _returnvalue _newtrack_1) false false)
        (else
          (Transformation|SetWorldLocation (Variables|Default|GetSM_Plate02) (+ _returnvalue _newtrack_1) false false)
          (if (Math|Boolean|ANDBoolean (Variables|Default|GetIsPlate01) (Variables|Default|GetIsPlate02) (Variables|Default|GetIsPlate03))
            (Default|ActivatePlate (Variables|Default|GetFog))))))))

(event OnComponentEndOverlap(Box02)
  (params (OverlappedComponent :type Primitive%20Component%20Object%20Reference) (OtherActor :type Actor%20Object%20Reference) (OtherComp :type Primitive%20Component%20Object%20Reference) (OtherBodyIndex :type Integer))
  (bind _sm_plate02 (Variables|Default|GetSM_Plate02))
  (bind _returnvalue (Transformation|GetWorldLocation _sm_plate02))
  (Variables|Default|SetIsPlate02 false)
  (bind _newtrack_1 (Timeline|Timeline_0 Reverse)
    (:Update
      (if (Class|TimelineComponent|IsReversing (Variables|Default|GetTimeline_0))
        (Transformation|SetWorldLocation (Variables|Default|GetSM_Plate02) (- _returnvalue _newtrack_1) false false)
        (else
          (Transformation|SetWorldLocation (Variables|Default|GetSM_Plate02) (+ _returnvalue _newtrack_1) false false)
          (if (Math|Boolean|ANDBoolean (Variables|Default|GetIsPlate01) (Variables|Default|GetIsPlate02) (Variables|Default|GetIsPlate03))
            (Default|ActivatePlate (Variables|Default|GetFog))))))))

(event OnComponentBeginOverlap(Box01)
  (params (OverlappedComponent :type Primitive%20Component%20Object%20Reference) (OtherActor :type Actor%20Object%20Reference) (OtherComp :type Primitive%20Component%20Object%20Reference) (OtherBodyIndex :type Integer) (bFromSweep :type Boolean) (SweepResult :type Hit%20Result%20Structure%20%28by%20ref%29))
  (bind _sm_plate01 (Variables|Default|GetSM_Plate01))
  (bind _returnvalue (Transformation|GetWorldLocation _sm_plate01))
  (Variables|Default|SetIsPlate01 true)
  (bind _newtrack_1 (Timeline|Timeline_1 Play)
    (:Update
      (if (Class|TimelineComponent|IsReversing (Variables|Default|GetTimeline_1))
        (Transformation|SetWorldLocation (Variables|Default|GetSM_Plate01) (- _returnvalue _newtrack_1) false false)
        (else
          (Transformation|SetWorldLocation (Variables|Default|GetSM_Plate01) (+ _returnvalue _newtrack_1) false false)
          (if (Math|Boolean|ANDBoolean (Variables|Default|GetIsPlate01) (Variables|Default|GetIsPlate02) (Variables|Default|GetIsPlate03))
            (Default|ActivatePlate (Variables|Default|GetFog))))))))

(event OnComponentEndOverlap(Box01)
  (params (OverlappedComponent :type Primitive%20Component%20Object%20Reference) (OtherActor :type Actor%20Object%20Reference) (OtherComp :type Primitive%20Component%20Object%20Reference) (OtherBodyIndex :type Integer))
  (bind _sm_plate01 (Variables|Default|GetSM_Plate01))
  (bind _returnvalue (Transformation|GetWorldLocation _sm_plate01))
  (Variables|Default|SetIsPlate01 false)
  (bind _newtrack_1 (Timeline|Timeline_1 Reverse)
    (:Update
      (if (Class|TimelineComponent|IsReversing (Variables|Default|GetTimeline_1))
        (Transformation|SetWorldLocation (Variables|Default|GetSM_Plate01) (- _returnvalue _newtrack_1) false false)
        (else
          (Transformation|SetWorldLocation (Variables|Default|GetSM_Plate01) (+ _returnvalue _newtrack_1) false false)
          (if (Math|Boolean|ANDBoolean (Variables|Default|GetIsPlate01) (Variables|Default|GetIsPlate02) (Variables|Default|GetIsPlate03))
            (Default|ActivatePlate (Variables|Default|GetFog))))))))

(fn ConstructionScript)