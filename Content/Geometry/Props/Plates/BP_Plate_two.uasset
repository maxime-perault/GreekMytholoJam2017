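; Two-pressure-plate puzzle prop that triggers either Stairs or Fog when both plates are held down at once.
; Each trigger box counts overlaps, so its plate activates on the first entry and releases on the last exit, with Wwise sounds.
; Timelines move each plate mesh by per-update offsets, reversing on release.
; Forward updates check both pressed flags, then IsStairs selects stairs activation or fog activation with sound.
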(event OnComponentBeginOverlap(Box_two02)
  (params (OverlappedComponent :type Primitive%20Component%20Object%20Reference) (OtherActor :type Actor%20Object%20Reference) (OtherComp :type Primitive%20Component%20Object%20Reference) (OtherBodyIndex :type Integer) (bFromSweep :type Boolean) (SweepResult :type Hit%20Result%20Structure%20%28by%20ref%29))
  (bind _sm_plate_two02 (Variables|Default|GetSM_Plate_two02))
  (bind _returnvalue (Transformation|GetWorldLocation _sm_plate_two02))
  (Variables|Default|SetNbPlayers01 (+ (Variables|Default|GetNbPlayers01) 1))
  (if (< (Variables|Default|GetNbPlayers01) 2)
    (Class|AkGameplayStatics|PostEventatLocation "/Game/Wwise/Play_sound_pressure.Play_sound_pressure" (Transformation|GetWorldLocation (Variables|Default|GetSM_Plate_two02)) "0, 0, 0")
    (Variables|Default|SetIsPlate02 true)
    (bind _newtrack_1 (Timeline|Timeline_0 Play)
      (:Update
        (if (Class|TimelineComponent|IsReversing (Variables|Default|GetTimeline_0))
          (Transformation|SetWorldLocation (Variables|Default|GetSM_Plate_two02) (- _returnvalue _newtrack_1) false false)
          (else
            (Transformation|SetWorldLocation (Variables|Default|GetSM_Plate_two02) (+ _returnvalue _newtrack_1) false false)
            (if (and (Variables|Default|GetIsPlate01) (Variables|Default|GetIsPlate02))
              (if (Variables|Default|GetisStairs)
                (Default|ActivateStairs (Variables|Default|GetStairs))
                (else
                  (Class|AkGameplayStatics|PostEvent "/Game/Wwise/Play_Fog.Play_Fog" self false)
                  (Default|ActivatePlate (Variables|Default|GetFog)))))))))))

(event OnComponentEndOverlap(Box_two02)
  (params (OverlappedComponent :type Primitive%20Component%20Object%20Reference) (OtherActor :type Actor%20Object%20Reference) (OtherComp :type Primitive%20Component%20Object%20Reference) (OtherBodyIndex :type Integer))
  (bind _sm_plate_two02 (Variables|Default|GetSM_Plate_two02))
  (bind _returnvalue (Transformation|GetWorldLocation _sm_plate_two02))
  (Variables|Default|SetNbPlayers01 (- (Variables|Default|GetNbPlayers01) 1))
  (if (== (Variables|Default|GetNbPlayers01) 0)
    (Class|AkGameplayStatics|PostEventatLocation "/Game/Wwise/Play_sound_depressure.Play_sound_depressure" (Transformation|GetWorldLocation (Variables|Default|GetSM_Plate_two02)) "0, 0, 0")
    (Variables|Default|SetIsPlate02 false)
    (bind _newtrack_1 (Timeline|Timeline_0 Reverse)
      (:Update
        (if (Class|TimelineComponent|IsReversing (Variables|Default|GetTimeline_0))
          (Transformation|SetWorldLocation (Variables|Default|GetSM_Plate_two02) (- _returnvalue _newtrack_1) false false)
          (else
            (Transformation|SetWorldLocation (Variables|Default|GetSM_Plate_two02) (+ _returnvalue _newtrack_1) false false)
            (if (and (Variables|Default|GetIsPlate01) (Variables|Default|GetIsPlate02))
              (if (Variables|Default|GetisStairs)
                (Default|ActivateStairs (Variables|Default|GetStairs))
                (else
                  (Class|AkGameplayStatics|PostEvent "/Game/Wwise/Play_Fog.Play_Fog" self false)
                  (Default|ActivatePlate (Variables|Default|GetFog)))))))))))

(event OnComponentBeginOverlap(Box_two01)
  (params (OverlappedComponent :type Primitive%20Component%20Object%20Reference) (OtherActor :type Actor%20Object%20Reference) (OtherComp :type Primitive%20Component%20Object%20Reference) (OtherBodyIndex :type Integer) (bFromSweep :type Boolean) (SweepResult :type Hit%20Result%20Structure%20%28by%20ref%29))
  (bind _sm_plate_two01 (Variables|Default|GetSM_Plate_two01))
  (bind _returnvalue (Transformation|GetWorldLocation _sm_plate_two01))
  (Variables|Default|SetNbPlayers02 (+ (Variables|Default|GetNbPlayers02) 1))
  (if (< (Variables|Default|GetNbPlayers02) 2)
    (Class|AkGameplayStatics|PostEventatLocation "/Game/Wwise/Play_sound_pressure.Play_sound_pressure" (Transformation|GetWorldLocation (Variables|Default|GetSM_Plate_two01)) "0, 0, 0")
    (Variables|Default|SetIsPlate01 true)
    (bind _newtrack_1 (Timeline|Timeline_1 Play)
      (:Update
        (if (Class|TimelineComponent|IsReversing (Variables|Default|GetTimeline_1))
          (Transformation|SetWorldLocation (Variables|Default|GetSM_Plate_two01) (- _returnvalue _newtrack_1) false false)
          (else
            (Transformation|SetWorldLocation (Variables|Default|GetSM_Plate_two01) (+ _returnvalue _newtrack_1) false false)
            (if (and (Variables|Default|GetIsPlate01) (Variables|Default|GetIsPlate02))
              (if (Variables|Default|GetisStairs)
                (Default|ActivateStairs (Variables|Default|GetStairs))
                (else
                  (Class|AkGameplayStatics|PostEvent "/Game/Wwise/Play_Fog.Play_Fog" self false)
                  (Default|ActivatePlate (Variables|Default|GetFog)))))))))))

(event OnComponentEndOverlap(Box_two01)
  (params (OverlappedComponent :type Primitive%20Component%20Object%20Reference) (OtherActor :type Actor%20Object%20Reference) (OtherComp :type Primitive%20Component%20Object%20Reference) (OtherBodyIndex :type Integer))
  (bind _sm_plate_two01 (Variables|Default|GetSM_Plate_two01))
  (bind _returnvalue (Transformation|GetWorldLocation _sm_plate_two01))
  (Variables|Default|SetNbPlayers02 (- (Variables|Default|GetNbPlayers02) 1))
  (if (== (Variables|Default|GetNbPlayers02) 0)
    (Class|AkGameplayStatics|PostEventatLocation "/Game/Wwise/Play_sound_depressure.Play_sound_depressure" (Transformation|GetWorldLocation (Variables|Default|GetSM_Plate_two01)) "0, 0, 0")
    (Variables|Default|SetIsPlate01 false)
    (bind _newtrack_1 (Timeline|Timeline_1 Reverse)
      (:Update
        (if (Class|TimelineComponent|IsReversing (Variables|Default|GetTimeline_1))
          (Transformation|SetWorldLocation (Variables|Default|GetSM_Plate_two01) (- _returnvalue _newtrack_1) false false)
          (else
            (Transformation|SetWorldLocation (Variables|Default|GetSM_Plate_two01) (+ _returnvalue _newtrack_1) false false)
            (if (and (Variables|Default|GetIsPlate01) (Variables|Default|GetIsPlate02))
              (if (Variables|Default|GetisStairs)
                (Default|ActivateStairs (Variables|Default|GetStairs))
                (else
                  (Class|AkGameplayStatics|PostEvent "/Game/Wwise/Play_Fog.Play_Fog" self false)
                  (Default|ActivatePlate (Variables|Default|GetFog)))))))))))

(fn ConstructionScript)