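; Double pressure-plate prop that activates a referenced Fog object when both plates are triggered together.
; Each box overlap plays a timeline that moves its plate mesh, and ending the overlap reverses it.
; Timeline values are added to or subtracted from the current world location every update, so movement is cumulative.
; Forward updates set that plate's flag and call ActivatePlate on Fog while both are true; reversing clears it.
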(event OnComponentBeginOverlap(Box02)
  (params (OverlappedComponent :type Primitive%20Component%20Object%20Reference) (OtherActor :type Actor%20Object%20Reference) (OtherComp :type Primitive%20Component%20Object%20Reference) (OtherBodyIndex :type Integer) (bFromSweep :type Boolean) (SweepResult :type Hit%20Result%20Structure%20%28by%20ref%29))
  (bind _sm_plate_double02 (Variables|Default|GetSM_Plate_double02))
  (bind _returnvalue (Transformation|GetWorldLocation _sm_plate_double02))
  (bind _newtrack_1 (Timeline|Timeline_0 Play)
    (:Update
      (if (Class|TimelineComponent|IsReversing (Variables|Default|GetTimeline_0))
        (Transformation|SetWorldLocation (Variables|Default|GetSM_Plate_double02) (- _returnvalue _newtrack_1) false false)
        (Variables|Default|SetIsPlate01 false)
        (else
          (Transformation|SetWorldLocation (Variables|Default|GetSM_Plate_double02) (+ _returnvalue _newtrack_1) false false)
          (bind _output_get (Variables|Default|SetIsPlate01 true))
          (if (and _output_get (stale OnComponentBeginOverlap(Box01) _output_get))
            (Default|ActivatePlate (Variables|Default|GetFog))))))))

(event OnComponentEndOverlap(Box02)
  (params (OverlappedComponent :type Primitive%20Component%20Object%20Reference) (OtherActor :type Actor%20Object%20Reference) (OtherComp :type Primitive%20Component%20Object%20Reference) (OtherBodyIndex :type Integer))
  (bind _sm_plate_double02 (Variables|Default|GetSM_Plate_double02))
  (bind _returnvalue (Transformation|GetWorldLocation _sm_plate_double02))
  (bind _newtrack_1 (Timeline|Timeline_0 Reverse)
    (:Update
      (if (Class|TimelineComponent|IsReversing (Variables|Default|GetTimeline_0))
        (Transformation|SetWorldLocation (Variables|Default|GetSM_Plate_double02) (- _returnvalue _newtrack_1) false false)
        (Variables|Default|SetIsPlate01 false)
        (else
          (Transformation|SetWorldLocation (Variables|Default|GetSM_Plate_double02) (+ _returnvalue _newtrack_1) false false)
          (bind _output_get (Variables|Default|SetIsPlate01 true))
          (if (and _output_get (stale OnComponentBeginOverlap(Box01) _output_get))
            (Default|ActivatePlate (Variables|Default|GetFog))))))))

(event OnComponentBeginOverlap(Box01)
  (params (OverlappedComponent :type Primitive%20Component%20Object%20Reference) (OtherActor :type Actor%20Object%20Reference) (OtherComp :type Primitive%20Component%20Object%20Reference) (OtherBodyIndex :type Integer) (bFromSweep :type Boolean) (SweepResult :type Hit%20Result%20Structure%20%28by%20ref%29))
  (bind _sm_plate_double01 (Variables|Default|GetSM_Plate_double01))
  (bind _returnvalue (Transformation|GetWorldLocation _sm_plate_double01))
  (bind _newtrack_1 (Timeline|Timeline_1 Play)
    (:Update
      (if (Class|TimelineComponent|IsReversing (Variables|Default|GetTimeline_1))
        (Transformation|SetWorldLocation (Variables|Default|GetSM_Plate_double01) (- _returnvalue _newtrack_1) false false)
        (Variables|Default|SetIsPlate02 false)
        (else
          (Transformation|SetWorldLocation (Variables|Default|GetSM_Plate_double01) (+ _returnvalue _newtrack_1) false false)
          (bind _output_get (Variables|Default|SetIsPlate02 true))
          (if (and (stale OnComponentBeginOverlap(Box02) _output_get) _output_get)
            (Default|ActivatePlate (Variables|Default|GetFog))))))))

(event OnComponentEndOverlap(Box01)
  (params (OverlappedComponent :type Primitive%20Component%20Object%20Reference) (OtherActor :type Actor%20Object%20Reference) (OtherComp :type Primitive%20Component%20Object%20Reference) (OtherBodyIndex :type Integer))
  (bind _sm_plate_double01 (Variables|Default|GetSM_Plate_double01))
  (bind _returnvalue (Transformation|GetWorldLocation _sm_plate_double01))
  (bind _newtrack_1 (Timeline|Timeline_1 Reverse)
    (:Update
      (if (Class|TimelineComponent|IsReversing (Variables|Default|GetTimeline_1))
        (Transformation|SetWorldLocation (Variables|Default|GetSM_Plate_double01) (- _returnvalue _newtrack_1) false false)
        (Variables|Default|SetIsPlate02 false)
        (else
          (Transformation|SetWorldLocation (Variables|Default|GetSM_Plate_double01) (+ _returnvalue _newtrack_1) false false)
          (bind _output_get (Variables|Default|SetIsPlate02 true))
          (if (and (stale OnComponentBeginOverlap(Box02) _output_get) _output_get)
            (Default|ActivatePlate (Variables|Default|GetFog))))))))

(fn ConstructionScript)