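; Pressure plate prop that activates a linked Fog while occupied and deactivates it once empty.
; A Box trigger counts overlaps in NbPlayers, so only the first arrival and last departure switch the Fog and post Wwise press or release sounds at the plate.
; Those events play or reverse a Timeline whose vector track is added to or subtracted from the mesh's world location each update, accumulating rather than interpolating between fixed positions.
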(event OnComponentBeginOverlap(Box)
  (params (OverlappedComponent :type Primitive%20Component%20Object%20Reference) (OtherActor :type Actor%20Object%20Reference) (OtherComp :type Primitive%20Component%20Object%20Reference) (OtherBodyIndex :type Integer) (bFromSweep :type Boolean) (SweepResult :type Hit%20Result%20Structure%20%28by%20ref%29))
  (bind _sm_plate_solo (Variables|Default|GetSM_Plate_solo))
  (bind _returnvalue (Transformation|GetWorldLocation _sm_plate_solo))
  (Variables|Default|Setnb_players (+ (Variables|Default|Getnb_players) 1))
  (if (< (Variables|Default|Getnb_players) 2)
    (Default|ActivatePlate (Variables|Default|GetFog))
    (Class|AkGameplayStatics|PostEventatLocation "/Game/Wwise/Play_sound_pressure.Play_sound_pressure" (Transformation|GetWorldLocation (Variables|Default|GetSM_Plate_solo)) "0, 0, 0")
    (bind _newtrack_1 (Timeline|Timeline_0 Play)
      (:Update
        (if (Class|TimelineComponent|IsReversing (Variables|Default|GetTimeline_0))
          (Transformation|SetWorldLocation (Variables|Default|GetSM_Plate_solo) (- _returnvalue _newtrack_1) false false)
          (else
            (Transformation|SetWorldLocation (Variables|Default|GetSM_Plate_solo) (+ _returnvalue _newtrack_1) false false)))))))

(event OnComponentEndOverlap(Box)
  (params (OverlappedComponent :type Primitive%20Component%20Object%20Reference) (OtherActor :type Actor%20Object%20Reference) (OtherComp :type Primitive%20Component%20Object%20Reference) (OtherBodyIndex :type Integer))
  (bind _sm_plate_solo (Variables|Default|GetSM_Plate_solo))
  (bind _returnvalue (Transformation|GetWorldLocation _sm_plate_solo))
  (Variables|Default|Setnb_players (- (Variables|Default|Getnb_players) 1))
  (if (== (Variables|Default|Getnb_players) 0)
    (Default|DesactivatePlate (Variables|Default|GetFog))
    (Class|AkGameplayStatics|PostEventatLocation "/Game/Wwise/Play_sound_depressure.Play_sound_depressure" (Transformation|GetWorldLocation (Variables|Default|GetSM_Plate_solo)) "0, 0, 0")
    (bind _newtrack_1 (Timeline|Timeline_0 Reverse)
      (:Update
        (if (Class|TimelineComponent|IsReversing (Variables|Default|GetTimeline_0))
          (Transformation|SetWorldLocation (Variables|Default|GetSM_Plate_solo) (- _returnvalue _newtrack_1) false false)
          (else
            (Transformation|SetWorldLocation (Variables|Default|GetSM_Plate_solo) (+ _returnvalue _newtrack_1) false false)))))))

(fn ConstructionScript)