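; BP_Cariatide_two is a prop Blueprint for a pair of caryatid statues that can switch to weeping versions and activate a fog plate.
; Each of two chains hides a normal statue mesh, shows its weeping counterpart, then joins a shared check that calls ActivatePlate on Fog once both weeping meshes are visible.
; No event triggers either chain, so this logic never runs as wired, and the construction script is empty.
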(fn ConstructionScript)