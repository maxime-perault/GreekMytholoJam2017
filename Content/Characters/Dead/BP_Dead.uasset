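; BP_Dead is an AI "Dead" character that Interact partitions enable or disable, with sound and an animation blend through ABP_Dead.
; Enabling turns on collision overlaps and stops movement, nudging the collision to sweep.
; Disabling resumes FollowPath: it heads to a valid Tree, otherwise walks PathPoints in order.
; At path end it loops, or notifies the Player, waits, and teleports to the first point to restart.
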(event Custom|FollowPath
  (bind _pathpoints (Variables|Dead|GetPathPoints))
  (bind _output (Utilities|Array|Get(acopy) _pathpoints))
  (bind _returnvalue (Transformation|GetActorLocation _output))
  (CallFunction|NotifyPlayer)
  (AI|Navigation|StopMovement (AI|GetAIController self))
  (Utilities|IsValid (Variables|Dead|GetTree)
    (:Is%20Valid
      (if (not (Variables|Dead|Getenabled))
        (AI|AIMoveTo (AI|GetAIController self) "0, 0, 0" (Variables|Dead|GetTree) -1.0 "Default" "Enable" true true
          (:then
            (Development|PrintString "GoesToTree" true true "(R=0.665213,G=0.000000,B=1.000000,A=1.000000)"))
          (:OnRequestFailed
            (AI|Navigation|StopMovement (AI|GetAIController self) :!label _label))
          (:OnMoveFinished
            (Development|PrintString "TreeFinished" true true "(R=0.665213,G=0.000000,B=1.000000,A=1.000000)")
            (goto _label)))))
    (:Is%20Not%20Valid
      (if (not (Variables|Dead|Getenabled))
        (if (> (Utilities|Array|Length (Variables|Dead|GetPathPoints)) 0)
          (AI|AIMoveTo (AI|GetAIController self) "0, 0, 0" (Utilities|Array|Get(acopy) (Variables|Dead|GetPathPoints) (Variables|Dead|GetCurrentPathPoint)) -1.0 "Default" "Default" true true :!label _label_2
            (:OnMoveFinished
              (Utilities|IsValid (Variables|Dead|GetTree)
                (:Is%20Not%20Valid
                  (if (not (Variables|Dead|Getenabled))
                    (if (> (Utilities|Array|Length (Variables|Dead|GetPathPoints)) (+ (Variables|Dead|GetCurrentPathPoint) 1))
                      (Variables|Dead|SetCurrentPathPoint (+ (Variables|Dead|GetCurrentPathPoint) 1))
                      (goto _label_2)
                      (else
                        (Variables|Dead|SetCurrentPathPoint 0)
                        (if (Variables|Dead|Getloop)
                          (goto _label_2)
                          (else
                            (CallFunction|NotifyPlayer)
                            (Utilities|FlowControl|Delay (Variables|Dead|GetrespawnDelay))
                            (Transformation|Teleport self _returnvalue (Math|Rotator|MakeRotator 0.0 0.0 (.yaw (Math|Rotator|FindLookatRotation _returnvalue (Transformation|GetActorLocation (Utilities|Array|Get(acopy) _pathpoints 1))))))
                            (CallFunction|FollowPath)))))))))))))))

(event EventInteract
  (params (Partition :type PartitionIDs%20Enum :default "NewEnumerator0"))
  (bind _self self)
  (switch Utilities|FlowControl|Switch|SwitchonPartitionIDs Partition
    (:NewEnumerator0
      (Class|AkGameplayStatics|PostEvent "/Game/Wwise/Play_sound_dead_activated.Play_sound_dead_activated" _self false)
      (CallFunction|SetEnabled true)
      (bind _alpha (Timeline|Timeline_Activation Play)
        (:Update
          (Variables|/Game/Characters/Dead/ABP_Dead.ABP_Dead_C|SetActivation%20Amount (.AsABP%20Dead (Utilities|Casting|CastToABP_Dead (Components|SkeletalMesh|GetAnimInstance (Variables|Default|GetDead_2)))) (* 1e+02 _alpha)))))
    (:NewEnumerator1
      (Class|AkGameplayStatics|PostEvent "/Game/Wwise/Play_sound_dead_disactivated.Play_sound_dead_disactivated" _self false)
      (CallFunction|SetEnabled false)
      (Timeline|Timeline_Activation Reverse))))

(event EventBeginPlay
  (bind _enabled (Variables|Dead|Getenabled))
  (Components|Timeline|SetPlayRate (Variables|Default|GetTimeline_Activation) (/ 1.0 (Variables|Dead|GetAnimationDuration)))
  (CallFunction|SetEnabled _enabled)
  (if _enabled
    (bind _alpha (Timeline|Timeline_Activation Play)
      (:Update
        (Variables|/Game/Characters/Dead/ABP_Dead.ABP_Dead_C|SetActivation%20Amount (.AsABP%20Dead (Utilities|Casting|CastToABP_Dead (Components|SkeletalMesh|GetAnimInstance (Variables|Default|GetDead_2)))) (* 1e+02 _alpha))))
    (else
      (Timeline|Timeline_Activation Reverse))))

(fn ConstructionScript)

(fn NotifyPlayer
  (bind _player (Variables|Default|GetPlayer))
  (Utilities|IsValid _player
    (:Is%20Valid
      (Default|DeadRespawned _player self))
    (:Is%20Not%20Valid
      _))
  (return))

(fn SetEnabled
  (params (enabled :type Boolean))
  (bind _output_get (Variables|Dead|Setenabled enabled))
  (bind _output_get_2 (Variables|/Script/Engine.PrimitiveComponent|SetbGenerateOverlapEvents (Variables|Default|GetEnabledCollision) _output_get))
  (Transformation|AddRelativeLocation (Variables|Default|GetEnabledCollision) (Math|Vector|MakeVector 0.0 0.0 (Math|Float|SelectFloat 0.01 -0.01 _output_get_2)) true false)
  (if _output_get_2
    (AI|Navigation|StopMovement (AI|GetAIController self))
    (else
      (CallFunction|FollowPath))))

(fn CanInteract
  (return true))

(fn GetTarget
  (return (Variables|Collision|GetCapsuleComponent)))