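; BP_Puzzlos is an interactable actor, apparently a puzzle piece, labelled with the name of its Partition enum value.
; The construction script writes that name to a TextRender component.
; Interact returns whether the player's controlled pawn overlaps its Box and prints the actor name and result for debugging.
; The event graph holds only disabled placeholder events.
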(event EventBeginPlay)

(event Collision|EventActorBeginOverlap
  (params (OtherActor :type Actor%20Object%20Reference)))

(event EventTick
  (params (DeltaSeconds :type Float%20%28single-precision%29)))

(fn ConstructionScript
  (Rendering|Components|TextRender|SetText (Variables|Default|GetTextRender) (Utilities|Text|ToText(String) (Utilities|String|EnumtoString (Variables|Default|GetPartition)))))

(fn Interact
  (bind _returnvalue (Game|GetPlayerController 0))
  (bind _box (Variables|Default|GetBox))
  (bind _returnvalue_2 (Pawn|GetControlledPawn _returnvalue))
  (bind _returnvalue_3 (Collision|IsOverlappingActor _box _returnvalue_2 :!class /Script/Engine.PrimitiveComponent))
  (Development|PrintString (Utilities|String|Append "Interact with " (Utilities|GetDisplayName self) " : " (Utilities|String|ToString(Boolean) _returnvalue_3)))
  (return _returnvalue_3))