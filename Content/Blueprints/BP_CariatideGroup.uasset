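; BP_CariatideGroup coordinates a puzzle of caryatid statues that activates a linked Fog object when solved.
; On BeginPlay it registers itself as the Group on each statue in its Cariatides array.
; UpdateStatues takes the changed statue: a correct one triggers CheckAllEnabled, while a wrong one disables statues in a loop.
; CheckAllEnabled fails if any member is not both meant to be activated and enabled; success calls ActivatePlate on Fog.
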(event Custom|UpdateStatues
  (params (from :type BP%20Cariatide%20Object%20Reference))
  (if (Variables|/Game/Geometry/Props/Cariatide/BP_Cariatide.BP_Cariatide_C|GetShouldBeActivated from)
    (bind _allenabled (CallFunction|CheckAllEnabled))
    (if _allenabled
      (Default|ActivatePlate (Variables|Default|GetFog)))
    (else
      (for _array_element 0
        (Default|SetEnabled _array_element false)))))

(event EventBeginPlay
  (for _array_element (Variables|Default|GetCariatides)
    (Variables|/Game/Geometry/Props/Cariatide/BP_Cariatide.BP_Cariatide_C|SetGroup _array_element self)))

(fn ConstructionScript)

(fn CheckAllEnabled
  (bind _array_element (Utilities|Array|ForEachLoopwithBreak (Variables|Default|GetCariatides) :!label _label)
    (:LoopBody
      (if (not (and (Variables|/Game/Geometry/Props/Cariatide/BP_Cariatide.BP_Cariatide_C|GetShouldBeActivated _array_element) (Variables|/Game/Geometry/Props/Cariatide/BP_Cariatide.BP_Cariatide_C|Getenabled _array_element)))
        (LocalVariables|SetallEnabledLocal false)
        (goto _label Break)))
    (:Completed
      (return (LocalVariables|GetallEnabledLocal)))))