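; Interactable flower actor that plays a blossom animation when its Interact event fires.
; BeginPlay gathers seven flower components into an array.
; Interact sets the timeline's play rate from BlossomDuration, sets its time and plays it, with each update uniformly scaling every flower by the timeline alpha times FlowerScale.
; GetTarget is an empty stub.
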(event EventBeginPlay
  (Variables|Default|SetFlowers (Utilities|Array|MakeArray (Variables|Default|GetFlower0) (Variables|Default|GetFlower1) (Variables|Default|GetFlower2) (Variables|Default|GetFlower3) (Variables|Default|GetFlower4) (Variables|Default|GetFlower5) (Variables|Default|GetFlower6))))

(event Collision|EventActorBeginOverlap
  (params (OtherActor :type Actor%20Object%20Reference)))

(event EventTick
  (params (DeltaSeconds :type Float%20%28single-precision%29)))

(event EventInteract
  (params (Partition :type PartitionIDs%20Enum :default "NewEnumerator0"))
  (Components|Timeline|SetPlayRate (Variables|Default|GetTimeline_Blossom) (/ 1.0 (Variables|Default|GetBlossomDuration)))
  (Utilities|FlowControl|Sequence
    (:then_0
      (bind _alpha (Timeline|Timeline_Blossom SetNewTime)
        (:Update
          (for _array_element (Variables|Default|GetFlowers)
            (Transformation|SetRelativeScale3D _array_element (Math|Vector|MakeVector (* _alpha (Variables|Default|GetFlowerScale)) (* _alpha (Variables|Default|GetFlowerScale)) (* _alpha (Variables|Default|GetFlowerScale))))))))
    (:then_1
      (Timeline|Timeline_Blossom Play))))

(fn ConstructionScript)

(fn GetTarget
  (return 0))