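; Blueprint function library for musical partitions, the note sequences played with four directional sing buttons.
; Partition data is read from the PartitionsData table using the enum's string as row name, giving the button expected at an index.
; Display names come from a linear scan of data table rows matching the partition.
; Each sing button maps to a Wwise note event posted on a given actor.
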(fn PartitionfromID
  (params (PartitionID :type PartitionIDs%20Enum :default "NewEnumerator0"))
  (bind _returnvalue (Utilities|GetDataTableRow (LocalVariables|GetPartitionsData) (Utilities|String|StringToName (Utilities|String|EnumtoString PartitionID)))
    (:then
      (return _returnvalue))))

(fn GetSingButton
  (params (Partition :type PartitionIDs%20Enum :default "NewEnumerator0") (index :type Integer))
  (bind _partition (CallFunction|PartitionfromID Partition))
  (return (Utilities|Array|Get(acopy) (.inputs _partition) index)))

(fn GetUserFriendlyName
  (params (Partition :type PartitionIDs%20Enum :default "NewEnumerator0"))
  (bind _datatable (LocalVariables|GetDataTable))
  (bind _outrownames (DataTable|GetDataTableRowNames _datatable))
  (for _array_element _outrownames
    (bind _returnvalue (Utilities|GetDataTableRow _datatable _array_element)
      (:then
        (if (Utilities|Enum|Equal(Enum) Partition (.Partition (Utilities|Struct|BreakPartitionUserFriendlyName _returnvalue)))
          (return (.Name (Utilities|Struct|BreakPartitionUserFriendlyName _returnvalue)))))))
  (return ""))

(fn PlayNoteSound
  (params (Actor :type Actor%20Object%20Reference) (singButton :type SingButtons%20Enum :default "NewEnumerator0"))
  (Class|AkGameplayStatics|PostEvent (Utilities|Select :Index singButton :NewEnumerator0 "/Game/Wwise/Play_note_1_si.Play_note_1_si" :NewEnumerator1 "/Game/Wwise/Play_note_2_sol.Play_note_2_sol" :NewEnumerator2 "/Game/Wwise/Play_note_4_re.Play_note_4_re" :NewEnumerator3 "/Game/Wwise/Play_note_3_mi.Play_note_3_mi") Actor false))